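; Spawner actor that places Bow_enemy3_BP enemies at random points inside its SpawnVolume.
; The custom SpawnEnemy event counts every Bow_enemy3_BP actor in the world and spawns one more AI pawn only while that count is below MaxEnemies.
; Nothing in this graph calls SpawnEnemy, as BeginPlay, overlap and Tick are all empty.
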(event `SpawnEnemy`
  (bind _outactors (`GameplayStatics.GetAllActorsOfClass` "/Game/bow_enemy3_BP.bow_enemy3_BP_C"))
  (if (< (`KismetArrayLibrary.Array_Length` _outactors) (`self.Max Enemies`))
    (`AIBlueprintHelperLibrary.SpawnAIFromClass` "/Game/bow_enemy3_BP.bow_enemy3_BP_C" null (`KismetMathLibrary.RandomPointInBoundingBox` (`SceneComponent.K2_GetComponentLocation` (`self.Spawn_Volume`)) (`BoxComponent.GetScaledBoxExtent` (`self.Spawn_Volume`))))))

(fn `UserConstructionScript`)