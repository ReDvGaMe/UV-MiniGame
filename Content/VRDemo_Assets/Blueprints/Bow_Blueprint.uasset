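; VR bow actor that can be attached to a parent component or dropped with physics, and renders a drawable bowstring.
; UpdateString stretches two string meshes from hidden end markers to the pull position and triggers draw audio past a distance threshold.
; ReleaseString straightens the string and plays a fire sound once the startup delay has passed.
; Optional AutoRotation turns the bow mesh toward the pull point in a flattened plane, repositioning both ends.
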(event `self.ReceiveBeginPlay`
  (`PrimitiveComponent.SetCollisionEnabled` (`self.Sphere`) "NoCollision")
  (`|ExecutionSequence`
    (:`then_0`
      (`SceneComponent.K2_AttachTo` (`self.Sphere`) (`self.bow_A`) "None" "KeepRelativeOffset" true)
      (`SceneComponent.SetVisibility` (`self.end1`) false false)
      (`SceneComponent.SetVisibility` (`self.end2`) false false)
      (`self.ReleaseString`))
    (:`then_1`
      (`KismetSystemLibrary.Delay` 1.0)
      (set `self.BowAwake` true))
    (:`then_2`
      (goto _label_2 :!via `initvars`))))

(event `UpdateString_Copy`
  (params (Position :type "Vector Structure"))
  (bind _returnvalue (* 1.0 0.003))
  (bind _returnvalue_2 (`SceneComponent.K2_GetComponentLocation` (`self.end1`)))
  (bind _returnvalue_3 (`SceneComponent.K2_GetComponentLocation` (`self.end2`)))
  (bind _returnvalue_4 (* (+ (`SceneComponent.K2_GetComponentLocation` (`self.end1`)) (`SceneComponent.K2_GetComponentLocation` (`self.end2`))) 0.5))
  (`SceneComponent.K2_SetWorldTransform` (`self.string2`) (`KismetMathLibrary.MakeTransform` (* (+ _returnvalue_4 _returnvalue_3) 0.5) (`KismetMathLibrary.FindLookAtRotation` _returnvalue_4 _returnvalue_3) (`KismetMathLibrary.MakeVector` (* (`KismetMathLibrary.VSize` (- _returnvalue_4 _returnvalue_3)) 0.01) _returnvalue _returnvalue)) false false :!label _label)
  (`SceneComponent.K2_SetWorldTransform` (`self.string1`) (`KismetMathLibrary.MakeTransform` (* (+ _returnvalue_4 _returnvalue_2) 0.5) (`KismetMathLibrary.FindLookAtRotation` _returnvalue_4 _returnvalue_2) (`KismetMathLibrary.MakeVector` (* (`KismetMathLibrary.VSize` (- _returnvalue_4 _returnvalue_2)) 0.01) _returnvalue _returnvalue)) false false))

(event `self.Sphere.OnComponentBeginOverlap`
  (params (OverlappedComponent :type "PrimitiveComponent Object Reference") (OtherActor :type "Actor Object Reference") (OtherComp :type "PrimitiveComponent Object Reference") (OtherBodyIndex :type Integer) (bFromSweep :type Boolean) (SweepResult :type "HitResult Structure (by ref)"))
  (if (== OtherActor "/Game/VRDemo_Assets/Meshes/VR_Controller_Oriented.VR_Controller_Oriented")
    (`AddComponent|NODE_AddStaticMeshComponent-0`)))

(event `ReleaseString`
  (`|ExecutionSequence`
    (:`then_0`
      (goto _label))
    (:`then_1`
      (if (`self.BowAwake`)
        (`GameplayStatics.PlaySoundAtLocation` "/Game/VRDemo_Assets/Audio/bow_fire_Cue.bow_fire_Cue" (`SceneComponent.K2_GetComponentLocation` (`self.end2`)))))))

(event `UpdateString`
  (params (Position :type "Vector Structure"))
  (bind _returnvalue (* 1.0 0.003))
  (bind _returnvalue_2 (`SceneComponent.K2_GetComponentLocation` (`self.end2`)))
  (bind _returnvalue_3 (`SceneComponent.K2_GetComponentLocation` (`self.end1`)))
  (bind _returnvalue_4 (`KismetMathLibrary.VSize` (- Position _returnvalue_3)))
  (`|ExecutionSequence`
    (:`then_0`
      (if (`self.AutoRotate`)
        (`self.AutoRotation` Position :!label _label_2)))
    (:`then_1`
      (`SceneComponent.K2_SetWorldTransform` (`self.string2`) (`KismetMathLibrary.MakeTransform` (* (+ Position _returnvalue_2) 0.5) (`KismetMathLibrary.FindLookAtRotation` Position _returnvalue_2) (`KismetMathLibrary.MakeVector` (* (`KismetMathLibrary.VSize` (- Position _returnvalue_2)) 0.01) _returnvalue _returnvalue)) false false)
      (`SceneComponent.K2_SetWorldTransform` (`self.string1`) (`KismetMathLibrary.MakeTransform` (* (+ Position _returnvalue_3) 0.5) (`KismetMathLibrary.FindLookAtRotation` Position _returnvalue_3) (`KismetMathLibrary.MakeVector` (* _returnvalue_4 0.01) _returnvalue _returnvalue)) false false))
    (:`then_3`
      (`/Engine/EditorBlueprintResources/StandardMacros.CompareFloat` _returnvalue_4 500.0
        (:`>`
          ;[1 1 1] Bow pull audio
          (`/Engine/EditorBlueprintResources/StandardMacros.DoOnce` true
            (:`Completed`
              (`AudioComponent.Play` (`self.BowLoadAudio`) 0.0))))))))

(event `CustomEvent`
  (params (AttachTo :type "SceneComponent Object Reference"))
  (`PrimitiveComponent.SetSimulatePhysics` (`self.StaticMeshComponent`) false)
  (`SceneComponent.K2_AttachToComponent` (`self.K2_GetRootComponent`) AttachTo "None" "KeepWorld" "KeepWorld" "KeepWorld" false))

(event `CustomEvent_1`
  (`PrimitiveComponent.SetSimulatePhysics` (`self.StaticMeshComponent`) true)
  (`self.K2_DetachFromActor` "KeepWorld" "KeepWorld" "KeepWorld"))

(fn `UserConstructionScript`)